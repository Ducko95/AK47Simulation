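; Cartridge casing actor that carries a bullet, fires it and plays a sound when the casing drops.
; Construction picks the casing material from the equipped weapon, and BeginPlay spawns a BulletBP attached to the mesh's BulletSocket.
; Fire plays the shot at world origin, detaches the bullet and launches it with gravity-free physics and a world-X impulse.
; The first capsule hit plays a random drop sound.
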(event OnComponentHit(Capsule)
  (params (HitComponent :type Primitive%20Component%20Object%20Reference) (OtherActor :type Actor%20Object%20Reference) (OtherComp :type Primitive%20Component%20Object%20Reference) (NormalImpulse :type Vector :default "0, 0, 0") (Hit :type Hit%20Result%20Structure%20%28by%20ref%29))
  (Utilities|FlowControl|DoOnce false
    (:Completed
      (CallFunction|PlayRandomSound (Variables|Default|GetCasingDropSWs) (Transformation|GetActorLocation)))))

(event EventBeginPlay
  (bind _returnvalue (Utilities|Name|MakeLiteralName "BulletSocket"))
  (bind _staticmesh (Variables|Default|GetStaticMesh))
  (bind _returnvalue_2 (Game|SpawnActorfromClass "/Game/BluePrints/BulletBP.BulletBP_C" (Transformation|GetSocketTransform _staticmesh _returnvalue "RTS_World") "AlwaysSpawn" 0 0))
  (Transformation|AttachComponentToComponent _returnvalue_2 _staticmesh _returnvalue "SnapToTarget" "SnapToTarget" "SnapToTarget" true)
  (Variables|Default|SetSpawnedBulllet _returnvalue_2))

(fn ConstructionScript
  (bind _index (CallFunction|GetEquippedWeaponMaterial))
  (Rendering|Material|SetMaterial (Variables|Default|GetStaticMesh) 0 (Utilities|Array|Get(acopy) (Variables|Default|GetCasingMIs) _index)))

(fn Fire
  (bind _spawnedbulllet (Variables|Default|GetSpawnedBulllet))
  (bind _returnvalue (Actor|GetComponentbyClass _spawnedbulllet "/Script/Engine.CapsuleComponent"))
  (Audio|PlaySoundatLocation "/Game/Audio/Shot.Shot" "0, 0, 0" "0, 0, 0" 1.0 1.0 0.0 0 0 0)
  (Transformation|DetachFromActor _spawnedbulllet "KeepWorld" "KeepWorld" "KeepWorld")
  (Physics|SetSimulatePhysics _returnvalue true)
  (Physics|SetEnableGravity _returnvalue false)
  (Physics|AddImpulse _returnvalue "0.300000,0.000000,0.000000" "None" false))