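; AK-47 weapon Blueprint with animated slide, trigger, fire selector, magazine swapping, muzzle flash and material cycling.
; Timelines lerp AK47ABP bone values, and their finished dispatchers chain each mechanical step through temporarily bound events.
; Trigger pull fires the chambered cartridge; slide travel ejects it with physics and loads another from the magazine, repeating in the third fire mode while held.
; The first fire mode is safety, blocking trigger and slide.
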(event OnComponentBeginOverlap(MuzzleCollider)
  (params (OverlappedComponent :type Primitive%20Component%20Object%20Reference) (OtherActor :type Actor%20Object%20Reference) (OtherComp :type Primitive%20Component%20Object%20Reference) (OtherBodyIndex :type Integer) (bFromSweep :type Boolean) (SweepResult :type Hit%20Result%20Structure%20%28by%20ref%29))
  (Development|PrintString "boom" false false)
  (Effects|SpawnEmitterAttached "/Game/Muzzles/Particles/P_MuzzleFlash51.P_MuzzleFlash51" (Variables|Default|GetSkeletalMesh) "MuzzleSocket" "0, 0, 0" "0, 0, 0" "0.500000,0.500000,0.500000"))

(event Custom|AnimateSelector
  (params (StartPosition :type Float%20%28single-precision%29) (EndPosition :type Float%20%28single-precision%29) (PlayRate :type Float%20%28single-precision%29))
  (Components|Timeline|SetPlayRate (Variables|Default|GetSelectorTL) PlayRate)
  (bind _newtrack_0 (Timeline|SelectorTL PlayFromStart)
    (:Update
      (Variables|/Game/Ordnance/AK47ABP.AK47ABP_C|SetSelectorRotation (Variables|Default|GetAK47ABP) (Math|Float|Lerp StartPosition EndPosition _newtrack_0)))
    (:Finished
      (Default|CallAnimationSelectorFinished))))

(event Custom|AnimateRelease
  (params (StartPosition :type Float%20%28single-precision%29) (EndPosition :type Float%20%28single-precision%29) (PlayRate :type Float%20%28single-precision%29))
  (Components|Timeline|SetPlayRate (Variables|Default|GetReleaseTL) PlayRate)
  (bind _newtrack_0 (Timeline|ReleaseTL PlayFromStart)
    (:Update
      (Variables|/Game/Ordnance/AK47ABP.AK47ABP_C|SetReleaseRotation (Variables|Default|GetAK47ABP) (Math|Float|Lerp StartPosition EndPosition _newtrack_0)))
    (:Finished
      (Default|CallAnimationReleaseFinished))))

(event Custom|Cycle%20Materials
  (Math|Integer|IncrementInt (Variables|Default|GetMaterial)
    (:%20%20
      (if (== (Variables|Default|GetMaterial) 5)
        (bind _output_get (Variables|Default|SetMaterial 0)))
      (CallFunction|ChangeMaterial _output_get))))

(event Custom|Drop%20Magazine
  (if (Variables|Default|GetMagazineAttached?)
    (CallFunction|AnimateRelease (Variables|/Game/Ordnance/AK47ABP.AK47ABP_C|GetReleaseRotation (Variables|Default|GetAK47ABP)) -2e+01 1e+01)
    (EventDispatchers|BindEventtoAnimationReleaseFinished (delegate Custom|After05))))

(event Custom|Cycle%20Selector
  (CallFunction|CycleFireMode)
  (CallFunction|MoveSelector))

(event Custom|After03
  (EventDispatchers|UnbindallEventsfromAnimationSlideFinished)
  (if (Math|Float|NearlyEqual(Float) (Variables|/Game/Ordnance/AK47ABP.AK47ABP_C|GetSlideTranslation (Variables|Default|GetAK47ABP)) -5.4 1e-06)
    (CallFunction|EjectandLoadCasing)))

(event Custom|Move%20Selector
  (bind _ak47abp (Variables|Default|GetAK47ABP))
  (bind _selectorrotation (Variables|/Game/Ordnance/AK47ABP.AK47ABP_C|GetSelectorRotation _ak47abp))
  (switch int (Variables|Default|GetFireMode)
    (:0
      (bind _float_out (CallFunction|MakeTemporaryFloat 0.0))
      (CallFunction|AnimateSelector _selectorrotation _float_out 5.0))
    (:1
      (bind _float_out_2 (CallFunction|MakeTemporaryFloat -11.0))
      (CallFunction|AnimateSelector _selectorrotation _float_out_2 5.0))
    (:2
      (bind _float_out_3 (CallFunction|MakeTemporaryFloat -2e+01))
      (CallFunction|AnimateSelector _selectorrotation _float_out_3 5.0))))

(event Custom|After02
  (bind _ak47abp (Variables|Default|GetAK47ABP))
  (bind _slidetranslation (Variables|/Game/Ordnance/AK47ABP.AK47ABP_C|GetSlideTranslation _ak47abp))
  (EventDispatchers|UnbindallEventsfromAnimationSlideFinished)
  (if (Math|Float|NearlyEqual(Float) _slidetranslation 0.0 1e-06)
    (if (Variables|Default|GetMagazineAttached?)
      (if (Variables|Default|GetHeld?)
        (if (== (Variables|Default|GetFireMode) 2)
          (if (Variables|Default|GetChambered?)
            (if (Math|Float|NearlyEqual(Float) _slidetranslation 0.0 1e-06)
              (Default|Fire (Variables|Default|GetSpawnedCartridge))
              (CallFunction|AnimateSlide _slidetranslation -5.4 1e+01)
              (EventDispatchers|BindEventtoAnimationSlideFinished (delegate Custom|After04)))
            (else
              (Audio|PlaySoundatLocation "/Game/Audio/SafteyFire.SafteyFire" "0, 0, 0" "0, 0, 0" 1.0 1.0 0.0 0 0 0))))))))

(event Custom|After01
  (bind _ak47abp (Variables|Default|GetAK47ABP))
  (bind _slidetranslation (Variables|/Game/Ordnance/AK47ABP.AK47ABP_C|GetSlideTranslation _ak47abp))
  (EventDispatchers|UnbindallEventsfromAnimationTriggerFinished)
  (if (Math|Float|NearlyEqual(Float) (Variables|/Game/Ordnance/AK47ABP.AK47ABP_C|GetTriggerRotation _ak47abp) -4e+01 1e-06)
    (if (Variables|Default|GetChambered?)
      (if (Math|Float|NearlyEqual(Float) _slidetranslation 0.0 1e-06)
        (Default|Fire (Variables|Default|GetSpawnedCartridge))
        (CallFunction|AnimateSlide _slidetranslation -5.4 1e+01)
        (EventDispatchers|BindEventtoAnimationSlideFinished (delegate Custom|After04)))
      (else
        (Audio|PlaySoundatLocation "/Game/Audio/SafteyFire.SafteyFire" "0, 0, 0" "0, 0, 0" 1.0 1.0 0.0 0 0 0)))))

(event Custom|After06
  (bind _returnvalue (Utilities|Name|MakeLiteralName "MagazineSocket"))
  (bind _skeletalmesh (Variables|Default|GetSkeletalMesh))
  (bind _ak47abp (Variables|Default|GetAK47ABP))
  (bind _returnvalue_2 (Transformation|GetSocketTransform _skeletalmesh _returnvalue "RTS_World"))
  (bind _releaserotation (Variables|/Game/Ordnance/AK47ABP.AK47ABP_C|GetReleaseRotation _ak47abp))
  (bind _location (Math|Transform|BreakTransform _returnvalue_2))
  (EventDispatchers|UnbindallEventsfromAnimationReleaseFinished)
  (if (Math|Float|NearlyEqual(Float) _releaserotation -2e+01 1e-06)
    (Variables|Default|SetMagazineAttached? true)
    (bind _returnvalue_3 (Game|SpawnActorfromClass "/Game/BluePrints/MagazineBP.MagazineBP_C" (Math|Transform|MakeTransform (Math|Vector|MakeVector 0.0 0.0 (- (.z _location) 2e+01)) "24.000000,0.000000,0.000000" "0.040000,0.020000,0.130000") "AlwaysSpawn" 0 0))
    (bind _output_get (Variables|Default|SetSpawnedMagazine _returnvalue_3))
    (bind _newtrack_0 (Timeline|Linear01 PlayFromStart)
      (:Update
        (Transformation|SetActorLocation _output_get (Math|Vector|MakeVector (.x _location) (.y _location) (Math|Float|Lerp (.z (Transformation|GetActorLocation _output_get)) (.z _location) _newtrack_0)) false false))
      (:Finished
        (Transformation|AttachComponentToComponent _output_get 0 _returnvalue "SnapToTarget" "SnapToTarget" "SnapToTarget" false)
        (CallFunction|AnimateRelease _releaserotation 0.0 1e+01)))))

(event Custom|ReleaseTrigger
  (Variables|Default|SetHeld? false)
  (Utilities|Safety ; enters at In (Silent)
    (:Saftey%20Off
      (CallFunction|AnimateTrigger (Variables|/Game/Ordnance/AK47ABP.AK47ABP_C|GetTriggerRotation (Variables|Default|GetAK47ABP)) 0.0 2e+01))))

(event Custom|After05
  (bind _ak47abp (Variables|Default|GetAK47ABP))
  (bind _spawnedmagazine (Variables|Default|GetSpawnedMagazine))
  (bind _returnvalue (Actor|GetComponentbyClass _spawnedmagazine "/Script/Engine.BoxComponent"))
  (bind _releaserotation (Variables|/Game/Ordnance/AK47ABP.AK47ABP_C|GetReleaseRotation _ak47abp))
  (EventDispatchers|UnbindallEventsfromAnimationReleaseFinished)
  (if (Math|Float|NearlyEqual(Float) _releaserotation -2e+01 1e-06)
    (Transformation|DetachFromComponent (Variables|/Script/Engine.Actor|GetRootComponent _spawnedmagazine) "KeepRelative" "KeepRelative" "KeepRelative" false)
    (Collision|SetCollisionEnabled _returnvalue "QueryAndPhysics")
    (Physics|SetSimulatePhysics _returnvalue true)
    (Physics|SetEnableGravity _returnvalue true)
    (Variables|Default|SetMagazineAttached? false)
    (CallFunction|AnimateRelease _releaserotation 0.0 1e+01)))

(event Custom|After04
  (bind _ak47abp (Variables|Default|GetAK47ABP))
  (bind _slidetranslation (Variables|/Game/Ordnance/AK47ABP.AK47ABP_C|GetSlideTranslation _ak47abp))
  (EventDispatchers|UnbindallEventsfromAnimationSlideFinished)
  (if (Math|Float|NearlyEqual(Float) _slidetranslation -5.4 1e-06)
    (CallFunction|EjectandLoadCasing)
    (CallFunction|AnimateSlide _slidetranslation 0.0 2e+01)
    (EventDispatchers|BindEventtoAnimationSlideFinished (delegate Custom|After02))))

(event Custom|PullTrigger
  (Variables|Default|SetHeld? true)
  (Utilities|Safety
    (:Saftey%20Off
      (CallFunction|AnimateTrigger (Variables|/Game/Ordnance/AK47ABP.AK47ABP_C|GetTriggerRotation (Variables|Default|GetAK47ABP)) -4e+01 2e+01)
      (EventDispatchers|BindEventtoAnimationTriggerFinished (delegate Custom|After01)))))

(event Custom|Pull%20Slide%20Back
  (Utilities|Safety
    (:Saftey%20Off
      (CallFunction|AnimateSlide (Variables|/Game/Ordnance/AK47ABP.AK47ABP_C|GetSlideTranslation (Variables|Default|GetAK47ABP)) -5.4 1e+01)
      (EventDispatchers|BindEventtoAnimationSlideFinished (delegate Custom|After03)))))

(event Custom|AnimateSlide
  (params (StartPosition :type Float%20%28single-precision%29) (EndPosition :type Float%20%28single-precision%29) (PlayRate :type Float%20%28single-precision%29))
  (if (>= StartPosition EndPosition)
    (Audio|PlaySoundatLocation "/Game/Audio/Slide1.Slide1" "0, 0, 0" "0, 0, 0" 1.0 1.0 0.0 0 0 0)
    (else
      (Audio|PlaySoundatLocation "/Game/Audio/Slide2.Slide2" "0, 0, 0" "0, 0, 0" 1.0 1.0 0.0 0 0 0)))
  (Components|Timeline|SetPlayRate (Variables|Default|GetSlideTL) PlayRate)
  (bind _newtrack_0 (Timeline|SlideTL PlayFromStart)
    (:Update
      (Variables|/Game/Ordnance/AK47ABP.AK47ABP_C|SetSlideTranslation (Variables|Default|GetAK47ABP) (Math|Float|Lerp StartPosition EndPosition _newtrack_0)))
    (:Finished
      (Default|CallAnimationSlideFinished))))

(event Custom|Release%20Slide
  (Utilities|Safety ; enters at In (Silent)
    (:Saftey%20Off
      (CallFunction|AnimateSlide (Variables|/Game/Ordnance/AK47ABP.AK47ABP_C|GetSlideTranslation (Variables|Default|GetAK47ABP)) 0.0 2e+01))))

(event Custom|AnimateTrigger
  (params (StartPosition :type Float%20%28single-precision%29) (EndPosition :type Float%20%28single-precision%29) (PlayRate :type Float%20%28single-precision%29))
  (Components|Timeline|SetPlayRate (Variables|Default|GetTriggerTL) PlayRate)
  (bind _newtrack_0 (Timeline|TriggerTL PlayFromStart)
    (:Update
      (Variables|/Game/Ordnance/AK47ABP.AK47ABP_C|SetTriggerRotation (Variables|Default|GetAK47ABP) (Math|Float|Lerp StartPosition EndPosition _newtrack_0)))
    (:Finished
      (Default|CallAnimationTriggerFinished))))

(event Custom|Insert%20New%20Magazine
  (Audio|PlaySoundatLocation "/Game/Audio/Reload.Reload" "0, 0, 0" "0, 0, 0" 1.0 1.0 0.0 0 0 0)
  (if (not (Variables|Default|GetMagazineAttached?))
    (CallFunction|AnimateRelease (Variables|/Game/Ordnance/AK47ABP.AK47ABP_C|GetReleaseRotation (Variables|Default|GetAK47ABP)) -2e+01 1e+01)
    (EventDispatchers|BindEventtoAnimationReleaseFinished (delegate Custom|After06))))

(event EventBeginPlay
  (bind _asak47abp (Utilities|Casting|CastToAK47ABP (Components|SkeletalMesh|GetAnimInstance (Variables|Default|GetSkeletalMesh))))
  (Variables|Default|SetAK47ABP _asak47abp))

(fn ConstructionScript)

(fn MakeTemporaryFloat
  (params (Float%20In :type Float%20%28single-precision%29))
  (return Float%20In))

(fn EjectandLoadCasing
  (bind _skeletalmesh (Variables|Default|GetSkeletalMesh))
  (if (Variables|Default|GetChambered?)
    (Transformation|DetachFromActor "KeepWorld" "KeepWorld" "KeepWorld")
    (Physics|SetSimulatePhysics (Actor|GetComponentbyClass (Variables|Default|GetSpawnedCartridge) "/Script/Engine.CapsuleComponent") true)
    (Physics|SetEnableGravity (Actor|GetComponentbyClass (Variables|Default|GetSpawnedCartridge) "/Script/Engine.CapsuleComponent") true)
    (Physics|AddImpulse (Actor|GetComponentbyClass (Variables|Default|GetSpawnedCartridge) "/Script/Engine.CapsuleComponent") (Math|Vector|MakeVector (Math|Random|RandomFloatinRange 0.1 0.2) (Math|Random|RandomFloatinRange 0.2 0.4) (Math|Random|RandomFloatinRange 0.0 0.1)) "None" false))
  (if (Variables|Default|GetMagazineAttached?)
    (if (> (Variables|/Game/BluePrints/MagazineBP.MagazineBP_C|GetBulletAmount (Variables|Default|GetSpawnedMagazine)) 0)
      (bind _returnvalue (Game|SpawnActorfromClass "/Game/BluePrints/CasingBP.CasingBP_C" (Transformation|GetSocketTransform _skeletalmesh "CasingSocket" "RTS_World") "AlwaysSpawn" 0 0))
      (bind _output_get (Variables|Default|SetSpawnedCartridge _returnvalue))
      (Transformation|AttachComponentToComponent _output_get _skeletalmesh "CasingSocket" "SnapToTarget" "SnapToTarget" "KeepRelative" true)
      (Variables|Default|SetChambered? true)
      (Default|TakeBullets (Variables|Default|GetSpawnedMagazine))
      (else
        (Variables|Default|SetChambered? false :!label _label)))
    (else
      (goto _label))))

(fn ChangeMaterial
  (params (Index :type Integer))
  (bind _output_get (Variables|Default|SetMaterial Index))
  (Rendering|Material|SetMaterial (Variables|Default|GetSkeletalMesh) 0 (Utilities|Array|Get(acopy) (Variables|Default|GetAK47MIs) _output_get)))

(fn CycleFireMode
  (if (not (Variables|Default|GetHeld?))
    (Audio|PlaySoundatLocation "/Game/Audio/SelectorChange.SelectorChange" "0, 0, 0" "0, 0, 0" 1.0 1.0 0.0 0 0 0)
    (switch int (Variables|Default|GetFireMode)
      (:0
        (Variables|Default|SetFireModeDirection 1))
      (:1
        _)
      (:2
        (bind _output_get (Variables|Default|SetFireModeDirection -1))))
    (bind _output_get_2 (Variables|Default|SetFireMode (+ _output_get (Variables|Default|GetFireMode))))
    (return _output_get_2)))