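; Helpers is a function library of shared lookups for an AK47 weapon setup plus a random sound utility.
; It finds the equipped weapon and camera by taking the first actor of the AK47BP and AK47Camera classes in the world.
; Weapon material and attached magazine bullet count are read through that weapon lookup.
; PlayRandomSound plays a random entry from a sound array at a given location.
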(fn PlayRandomSound
  (params (Sounds :type Array%20of%20Sound%20Wave%20Object%20References) (Location :type Vector))
  (Audio|PlaySoundatLocation 0 (Utilities|Array|Get(acopy) Sounds (Math|Random|RandomIntegerinRange 0 (- (Utilities|Array|Length Sounds) 1))) Location "0, 0, 0" 1.0 1.0 0.0 0 0 0))

(fn GetEquippedWeaponMaterial
  (bind _equppiedweapon (CallFunction|GetEquippedWeapon))
  (return (Variables|/Game/BluePrints/AK47BP.AK47BP_C|GetMaterial _equppiedweapon)))

(fn GetEquippedWeapon
  (bind _outactors (Actor|GetAllActorsOfClass 0 "/Game/BluePrints/AK47BP.AK47BP_C"))
  (return (Utilities|Array|Get(acopy) _outactors)))

(fn GetCamera
  (bind _outactors (Actor|GetAllActorsOfClass 0 "/Game/BluePrints/AK47Camera.AK47Camera_C"))
  (return (Utilities|Array|Get(acopy) _outactors)))

(fn GetAttachedMagazineBullets
  (bind _equppiedweapon (CallFunction|GetEquippedWeapon))
  (return (Variables|/Game/BluePrints/MagazineBP.MagazineBP_C|GetBulletAmount (Variables|/Game/BluePrints/AK47BP.AK47BP_C|GetSpawnedMagazine _equppiedweapon))))