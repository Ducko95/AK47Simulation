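; Weapon magazine actor that tracks its bullet count and picks its mesh material from the equipped weapon's material.
; On BeginPlay it spawns up to two casing actors attached to mesh sockets, showing only the top rounds rather than the full load.
; TakeBullets decrements the count and, below two, has UpdateBullets destroy surplus casings along with their bullets.
; The box's first hit plays a random magazine drop sound.
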(event OnComponentHit(Box)
  (params (HitComponent :type Primitive%20Component%20Object%20Reference) (OtherActor :type Actor%20Object%20Reference) (OtherComp :type Primitive%20Component%20Object%20Reference) (NormalImpulse :type Vector :default "0, 0, 0") (Hit :type Hit%20Result%20Structure%20%28by%20ref%29))
  (Utilities|FlowControl|DoOnce false
    (:Completed
      (CallFunction|PlayRandomSound (Variables|Default|GetMagazineDropSWs) (Transformation|GetActorLocation)))))

(event EventBeginPlay
  (CallFunction|ShowBullets))

(fn ConstructionScript
  (bind _index (CallFunction|GetEquippedWeaponMaterial))
  (Rendering|Material|SetMaterial (Variables|Default|GetStaticMesh) 0 (Utilities|Array|Get(acopy) (Variables|Default|GetMagazineMIs) _index)))

(fn ShowBullets
  (bind _staticmesh (Variables|Default|GetStaticMesh))
  (bind _bulletamount (Variables|Default|GetBulletAmount))
  (bind _spawnedcasings (Variables|Default|GetSpawnedCasings))
  (if (> _bulletamount 0)
    (bind _returnvalue (Game|SpawnActorfromClass "/Game/Ordnance/CasingBP.CasingBP_C" (Transformation|GetSocketTransform _staticmesh "CasingSocket2" "RTS_World") "AlwaysSpawn" 0 0))
    (Transformation|AttachComponentToComponent _returnvalue _staticmesh "CasingSocket1" "SnapToTarget" "SnapToTarget" "SnapToTarget" true)
    (Utilities|Array|Add _spawnedcasings _returnvalue)
    (if (> _bulletamount 1)
      (bind _returnvalue_2 (Game|SpawnActorfromClass "/Game/Ordnance/CasingBP.CasingBP_C" (Transformation|GetSocketTransform _staticmesh "CasingSocket1" "RTS_World") "AlwaysSpawn" 0 0))
      (Transformation|AttachComponentToComponent _returnvalue_2 _staticmesh "CasingSocket2" "SnapToTarget" "SnapToTarget" "SnapToTarget" true)
      (Utilities|Array|Add _spawnedcasings _returnvalue_2))))

(fn UpdateBullets
  (params (New%20Bullet%20Amount :type Integer))
  (bind _spawnedcasings (Variables|Default|GetSpawnedCasings))
  (bind (_array_element _array_index) (Utilities|Array|ForEachLoopwithBreak _spawnedcasings)
    (:LoopBody
      (if (> _array_index (- New%20Bullet%20Amount 1))
        (Actor|DestroyActor (Variables|/Game/Ordnance/CasingBP.CasingBP_C|GetSpawnedBulllet _array_element))
        (Actor|DestroyActor _array_element)
        (Utilities|Array|RemoveIndex _spawnedcasings _array_index)))))

(fn TakeBullets
  (if (> (Variables|Default|GetBulletAmount) 0)
    (bind _output_get (Variables|Default|SetBulletAmount (- (Variables|Default|GetBulletAmount) 1)))
    (if (< _output_get 2)
      (CallFunction|UpdateBullets _output_get))))